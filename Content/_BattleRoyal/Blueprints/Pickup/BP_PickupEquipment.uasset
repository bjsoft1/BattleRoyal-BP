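; BP_PickupEquipment is a battle royale equipment pickup configured from the DT_ItemEquipment data table by its row ID.
; The construction script reads the row and initializes the pickup's type, name, mesh and "SWITCH TO" prompt.
; Two equipment types, noted as backpack and bulletproof vest, get their mesh flattened and rotated.
; On BeginPlay the actor shifts up by its mesh's bounds height, doubled for one equipment type.
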(event `self.ReceiveBeginPlay`
  (bind (_origin _boxextent) (`KismetSystemLibrary.GetComponentBounds` (`self.StaticMesh`)))
  (`parent.ReceiveBeginPlay`)
  ;[1 1 1] Adjust the Static mesh INitial Position(Offset)
  (if (`|EnumEquality` (`self.equipmentType`) "NewEnumerator5")
    (`self.K2_AddActorLocalOffset` (`KismetMathLibrary.MakeVector` 0.0 0.0 (* (.z _boxextent) 2.0)))
    (else
      (`self.K2_AddActorLocalOffset` (`KismetMathLibrary.MakeVector` 0.0 0.0 (.z _boxextent))))))

(fn `UserConstructionScript`
  (bind (_datas_name _datas_type _datas_staticmesh) (break `/Game/_BattleRoyal/Blueprints/Data/Table/ST_ItemEquipment` (`self.datas`)))
  (bind _staticmesh (`self.StaticMesh`))
  (bind _staticmesh_2 (`self.StaticMesh`))
  (bind _returnvalue (`|GetDataTableRow` "/Game/_BattleRoyal/Blueprints/Data/Table/DT_ItemEquipment.DT_ItemEquipment" (`self.ID`))
    (:`then`
      (set `self.datas` _returnvalue)
      (set `self.equipmentType` _datas_type)
      (`self.InitilazePickup` _datas_type _datas_name "SWITCH TO " _datas_staticmesh)
      ;[1 1 1] Backpack And Bullet prof vest comes then change rotatin and scale
      (`|ExecutionSequence`
        (:`then_0`
          (if (`|EnumEquality` _datas_type "NewEnumerator6")
            (`SceneComponent.SetWorldScale3D` _staticmesh_2 (1.0 0.1 1.0))
            (`SceneComponent.K2_SetWorldRotation` _staticmesh_2 (struct :`Roll` -90.0) false true)))
        (:`then_1`
          (if (`|EnumEquality` _datas_type "NewEnumerator7")
            (`SceneComponent.SetWorldScale3D` _staticmesh (1.0 0.1 1.0))
            (`SceneComponent.K2_SetWorldRotation` _staticmesh (struct :`Roll` 90.0) false true)))))))