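; Usable health item pickup for the battle royale game, configured from the DT_ItemHealth data table.
; The construction script looks up the row by ID, caches it, passes item type and name to Initilaze, and copies the use time.
; GetWeight multiplies the amount by the row's per-item weight.
; The event graph holds only disabled stubs, so no healing logic appears here.
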(fn `GetWeight`
  (returns (Weight :type Integer))
  (bind (_datas_name _datas_staticmesh _datas_icon _datas_weight) (break `/Game/_BattleRoyal/Blueprints/Data/Table/ST_ItemHealth` (`self.datas`)))
  (return (* (`self.Amount`) _datas_weight)))

(fn `UserConstructionScript`
  (bind _returnvalue (`|GetDataTableRow` "/Game/_BattleRoyal/Blueprints/Data/Table/DT_ItemHealth.DT_ItemHealth" (`self.ID`))
    (:`then`
      (bind _output_get (set `self.datas` _returnvalue))
      (`self.Initilaze` "NewEnumerator3" (break `/Game/_BattleRoyal/Blueprints/Data/Table/ST_ItemHealth` _output_get))
      (set `self.useTime` (`.UseTime_14_C0A23BAF41A8B58F0E584EB961B0DF15` (break `/Game/_BattleRoyal/Blueprints/Data/Table/ST_ItemHealth` _output_get))))))