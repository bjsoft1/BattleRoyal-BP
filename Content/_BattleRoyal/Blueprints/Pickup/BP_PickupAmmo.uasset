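; BP_PickupAmmo is an ammo pickup for the battle royale mode, configured by a row ID.
; Its Construction Script looks up that ID in DT_AmmoItems, caches the unit weight and fills Amount from the row's default only when it is zero.
; It then passes the item type, name, "PICK UP" prompt and mesh to InitilazePickup.
; GetWeight returns unit weight times Amount, and the event graph holds no logic.
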(fn `GetWeight`
  (returns (Weight :type Integer))
  (return (* (`self.singleWeight`) (`self.Amount`))))

(fn `UserConstructionScript`
  (locals (datas :type "/Game/_BattleRoyal/Blueprints/Data/Table/ST_AmmoItems Structure"))
  (bind _returnvalue (`|GetDataTableRow` "/Game/_BattleRoyal/Blueprints/Data/Table/DT_AmmoItems.DT_AmmoItems" (`self.ID`))
    (:`then`
      (bind _output_get (set `local.datas` _returnvalue))
      (if (== (`self.Amount`) 0)
        (bind (_name _pickupmesh _pickupammo _icon _weight) (break `/Game/_BattleRoyal/Blueprints/Data/Table/ST_AmmoItems` _output_get))
        (set `self.Amount` _pickupammo))
      (set `self.singleWeight` _weight)
      (`self.InitilazePickup` "NewEnumerator2" _name "PICK UP " _pickupmesh))))