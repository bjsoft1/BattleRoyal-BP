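; BP_ItemBase is a base item Blueprint in the battle royale pickup system, holding an item's name, type and amount.
; On BeginPlay it casts and caches the first player's character and controller as owner references, regardless of who holds the item.
; Initilaze sets name and type, SetAmount increases, reduces or overwrites the amount through two flags, and GetWeight returns a placeholder zero.
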(event `self.ReceiveBeginPlay`
  ;[1 1 1] Try to set Character & Controller Refernce
  (bind _asbp_character (cast `/Game/_BattleRoyal/Blueprints/Character/BP_Character` (`GameplayStatics.GetPlayerCharacter` 0)))
  (set `self.OwnerCharacter` _asbp_character)
  (bind _asbp_player_controller (cast `/Game/_BattleRoyal/Blueprints/Game/BP_PlayerController` (`GameplayStatics.GetPlayerController` 0)))
  (set `self.OwnerController` _asbp_player_controller))

(fn `GetWeight`
  (returns (Weight :type Integer))
  (return 0))

(fn `Initilaze`
  (params (ItemType :type "/Game/_BattleRoyal/Blueprints/Data/Enum/E_ItemType Enum" :default "NewEnumerator0") (Name :type Text))
  (set `self.Name` Name)
  (set `self.ItemType` ItemType))

(fn `SetAmount`
  (params (IsIncressed :type Boolean) (IsReduce :type Boolean) (Amount :type Integer))
  (if IsIncressed
    (set `self.Amount` (+ Amount (`self.Amount`)))
    (elif IsReduce
      (set `self.Amount` (- (`self.Amount`) Amount))
      (else
        (set `self.Amount` Amount)))))

(fn `UserConstructionScript`)