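; Battle royale pickup actor for weapon accessories, configured per ID from DT_WeaponItemAccessories.
; The construction script looks up the row, stores its data and type, initializes the inherited pickup with name and mesh, and rotates foregrips, magazines and buttstocks to lie flat.
; BeginPlay lifts every type except sights by the mesh's Z bounds extent to correct its landing position.
; GetWeight reads the weight from the same table row.
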(event `self.ReceiveBeginPlay`
  (`parent.ReceiveBeginPlay`)
  ;[1 1 1] Adjust the model landing position
  (if (`|EnumInequality` (`self.AccessoriesType`) "NewEnumerator6")
    (`self.K2_AddActorLocalOffset` (`KismetMathLibrary.MakeVector` 0.0 0.0 (.z (`.BoxExtent` (`KismetSystemLibrary.GetComponentBounds` (`self.StaticMesh`))))))))

(fn `GetWeight`
  (returns (Weight :type Integer))
  (bind _returnvalue (`|GetDataTableRow` "/Game/_BattleRoyal/Blueprints/Data/Table/DT_WeaponItemAccessories.DT_WeaponItemAccessories" (`self.ID`))
    (:`then`
      (return (`.Weight_14_749510F14727D2A85CA6AD9B14876170` (break `/Game/_BattleRoyal/Blueprints/Data/Table/ST_WeaponItemAcc` _returnvalue))))))

(fn `UserConstructionScript`
  (bind _returnvalue (`|GetDataTableRow` "/Game/_BattleRoyal/Blueprints/Data/Table/DT_WeaponItemAccessories.DT_WeaponItemAccessories" (`self.ID`))
    (:`then`
      (bind _output_get (set `self.datas` _returnvalue))
      (bind (_name _type _weaponids _weight _staticmesh) (break `/Game/_BattleRoyal/Blueprints/Data/Table/ST_WeaponItemAcc` _output_get))
      (set `self.AccessoriesType` _type)
      (`self.InitilazePickup` "NewEnumerator1" _name "PICK UP " _staticmesh)
      ;[1 1 1] Auto Rotation when Need Rotation
      (switch `/Game/_BattleRoyal/Blueprints/Data/Enum/E_WeaponAccessoriesTypes` (`self.AccessoriesType`)
        (:`NewEnumerator1`
          _)
        (:`NewEnumerator2`
          _)
        (:`NewEnumerator3`
          _))
      (`SceneComponent.K2_SetWorldRotation` (`self.StaticMesh`) (struct :`Roll` -90.0) false false))))