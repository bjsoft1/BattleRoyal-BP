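; BP_PickupHealth is a health item pickup for the battle royale game, configured from a data table.
; The construction script looks up its ID in DT_ItemHealth, stores the row and unit weight, then initializes the pickup with item type, name, prompt prefix and static mesh.
; GetWeight returns the unit weight multiplied by Amount.
; The event graph holds no active logic.
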(fn `GetWeight`
  (returns (Weight :type Integer))
  (return (* (`self.singleWeight`) (`self.Amount`))))

(fn `UserConstructionScript`
  (bind _returnvalue (`|GetDataTableRow` "/Game/_BattleRoyal/Blueprints/Data/Table/DT_ItemHealth.DT_ItemHealth" (`self.ID`))
    (:`then`
      (bind _output_get (set `self.datas` _returnvalue))
      (bind (_name _staticmesh _icon _weight) (break `/Game/_BattleRoyal/Blueprints/Data/Table/ST_ItemHealth` _output_get))
      (set `self.singleWeight` _weight)
      (`self.InitilazePickup` "NewEnumerator3" _name "PICK UP " _staticmesh))))