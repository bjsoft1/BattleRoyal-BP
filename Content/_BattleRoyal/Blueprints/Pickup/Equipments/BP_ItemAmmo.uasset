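; Ammo pickup item for the battle royale game, configured from a data table.
; The construction script looks up its ID in DT_AmmoItems, caches the row in Datas, and passes the item type and name to Initilaze.
; GetWeight scales the row's unit weight by the stack Amount.
; The event graph holds only disabled stubs, so the Blueprint adds no runtime event logic.
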(fn `GetWeight`
  (returns (Weight :type Integer))
  (return (* (`.Weight_14_9043E8BB49D3A64F8DD31781EB98800D` (break `/Game/_BattleRoyal/Blueprints/Data/Table/ST_AmmoItems` (`self.datas`))) (`self.Amount`))))

(fn `UserConstructionScript`
  (bind _returnvalue (`|GetDataTableRow` "/Game/_BattleRoyal/Blueprints/Data/Table/DT_AmmoItems.DT_AmmoItems" (`self.ID`))
    (:`then`
      (bind _output_get (set `self.datas` _returnvalue))
      (`self.Initilaze` "NewEnumerator2" (`.Name_15_7C02B0664127F21F3705739D57C2D26A` (break `/Game/_BattleRoyal/Blueprints/Data/Table/ST_AmmoItems` _output_get))))))