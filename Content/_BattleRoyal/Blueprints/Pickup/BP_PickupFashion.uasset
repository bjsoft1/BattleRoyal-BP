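; Fashion item pickup for the battle royale game, representing an equippable clothing piece in the world.
; The construction script looks up its ID in DT_FashionItems, stores the fashion type and initializes the pickup with the row's name, mesh and an equip prompt.
; Every type except one (shoes, per the comment) is rotated and flattened.
; BeginPlay raises the actor by the mesh's vertical extent.
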(event `self.ReceiveBeginPlay`
  (`parent.ReceiveBeginPlay`)
  ;[1 1 1] Adjust the cloths initial location according to size
  (`self.K2_AddActorLocalOffset` (`KismetMathLibrary.MakeVector` 0.0 0.0 (.z (`.BoxExtent` (`KismetSystemLibrary.GetComponentBounds` (`self.StaticMesh`)))))))

(fn `UserConstructionScript`
  (bind _staticmesh (`self.StaticMesh`))
  (bind _returnvalue (`|GetDataTableRow` "/Game/_BattleRoyal/Blueprints/Data/Table/DT_FashionItems.DT_FashionItems" (`self.ID`))
    (:`then`
      (bind _output_get (set `self.datas` _returnvalue))
      (bind (_type _name _icon _skeletalmesh _staticmesh_2) (break `/Game/_BattleRoyal/Blueprints/Data/Table/ST_FashionTypes` _output_get))
      (set `self.fashionType` _type)
      (`self.InitilazePickup` "NewEnumerator8" _name "EQUIP " _staticmesh_2)
      ;[1 1 1] Change Size And rotion when not comes Shoes.
      (if (`|EnumInequality` _type "NewEnumerator3")
        (`SceneComponent.K2_SetWorldRotation` _staticmesh (struct :`Roll` -90.0) false false)
        (`SceneComponent.SetWorldScale3D` _staticmesh (1.0 0.1 1.0))))))