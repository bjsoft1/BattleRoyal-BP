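; Base pickup actor for a battle royale game that drops itself to the ground and highlights when its owner character is in range.
; BeginPlay traces downward for a specific object type and moves the pickup to the hit location.
; Box overlaps by OwnerCharacter fire begin and end overlap dispatchers and toggle a custom-depth outline on the mesh.
; InitilazePickup sets item type, name, UI prefix and static mesh.
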(event `self.ReceiveBeginPlay`
  (bind (_returnvalue_x _returnvalue_y _returnvalue_z) (`KismetMathLibrary.BreakVector` (`self.K2_GetActorLocation`)))
  (`parent.ReceiveBeginPlay`)
  ;[1 1 1] Pickup Fall to ground automatic
  (bind _outhit (`KismetSystemLibrary.LineTraceSingleForObjects` (`self.K2_GetActorLocation`) (`KismetMathLibrary.MakeVector` _returnvalue_x _returnvalue_y (+ _returnvalue_z -1000.0)) (`|MakeArray` "ObjectTypeQuery7" :!type "EObjectTypeQuery Enum")))
  (`self.K2_SetActorLocation` (`.Location` (`GameplayStatics.BreakHitResult` _outhit))))

(event `self.Box.OnComponentBeginOverlap`
  (params (OverlappedComponent :type "PrimitiveComponent Object Reference") (OtherActor :type "Actor Object Reference") (OtherComp :type "PrimitiveComponent Object Reference") (OtherBodyIndex :type Integer) (bFromSweep :type Boolean) (SweepResult :type "HitResult Structure (by ref)"))
  ;[1 1 1] Collision range check
  (if (== OtherActor (`self.OwnerCharacter`))
    (`self.OnBeginOverlapped` self)
    (`self.ShowOutLine` true)))

(event `self.Box.OnComponentEndOverlap`
  (params (OverlappedComponent :type "PrimitiveComponent Object Reference") (OtherActor :type "Actor Object Reference") (OtherComp :type "PrimitiveComponent Object Reference") (OtherBodyIndex :type Integer))
  ;[1 1 1] Collision range check
  (if (== OtherActor (`self.OwnerCharacter`))
    (`self.OnEndOverlapped` self)
    (`self.ShowOutLine` false)))

(fn `InitilazePickup`
  (params (itemType :type "/Game/_BattleRoyal/Blueprints/Data/Enum/E_ItemType Enum" :default "NewEnumerator0") (Name :type Text) (uiPrefix :type Text) (StaticMesh :type "StaticMesh Object Reference"))
  (`self.Initilaze` itemType Name)
  (set `self.UI_Prefix` uiPrefix)
  (`StaticMeshComponent.SetStaticMesh` (`self.StaticMesh`) StaticMesh))

(fn `ShowOutLine`
  (params (isEnabled :type Boolean))
  (bind _staticmesh (`self.StaticMesh`))
  (if isEnabled
    (`PrimitiveComponent.SetRenderCustomDepth` _staticmesh true)
    (else
      (`PrimitiveComponent.SetRenderCustomDepth` _staticmesh false))))

(fn `UserConstructionScript`)