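; Battle royale player controller that turns input into movement, look, jump, crouch and prone on BP_Character.
; Stance changes set data-table camera heights eased by timeline, clamp pitch per stance, and pause movement for prone transition times from DT_ProneTime.
; Holding Alt allows free look while movement keeps the saved heading; release lerps the view back.
; Max walk speed ramps from current velocity up to WalkSpeed.
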(event `UpdateCameraHeight`
  (bind _ownercharacter (`self.OwnerCharacter`))
  (bind _currentcameraheight (`self.currentCameraHeight`))
  (bind _cameraboom (`/Game/_BattleRoyal/Blueprints/Character/BP_Character.CameraBoom` _ownercharacter))
  (bind (_relativelocation_x _relativelocation_y) (`KismetMathLibrary.BreakVector` (`SceneComponent.RelativeLocation` _cameraboom)))
  (`|ExecutionSequence`
    (:`then_0`
      ;[1 1 1] Update Camera Height According to Character Position
      (if (`/Game/_BattleRoyal/Blueprints/Character/BP_Character.isCrouch` _ownercharacter)
        (if (and (not (`/Game/_BattleRoyal/Blueprints/Character/BP_Character.isHoldWeapon` _ownercharacter)) (or (!= (`self.moveForwardAxis`) 0.0) (!= (`self.moveRightAxis`) 0.0)))
          (bind _returnvalue (`|GetDataTableRow` "/Game/_BattleRoyal/Blueprints/Data/Table/DT_CameraHeight.DT_CameraHeight" "Crouch_Normal_Move")
            (:`then`
              (set `self.newCameraHeight` (`.Height_2_0FCAD2D647485573C84BE993991DC84C` (break `/Game/_BattleRoyal/Blueprints/Data/Table/ST_CameraHeight` _returnvalue)))))
          (elif (and (`/Game/_BattleRoyal/Blueprints/Character/BP_Character.isHoldWeapon` _ownercharacter) (or (!= (`self.moveForwardAxis`) 0.0) (!= (`self.moveRightAxis`) 0.0)))
            (bind _returnvalue_2 (`|GetDataTableRow` "/Game/_BattleRoyal/Blueprints/Data/Table/DT_CameraHeight.DT_CameraHeight" "Crouch_Rifle_Move")
              (:`then`
                (set `self.newCameraHeight` (`.Height_2_0FCAD2D647485573C84BE993991DC84C` (break `/Game/_BattleRoyal/Blueprints/Data/Table/ST_CameraHeight` _returnvalue_2)))))
            (else
              (bind _returnvalue_3 (`|GetDataTableRow` "/Game/_BattleRoyal/Blueprints/Data/Table/DT_CameraHeight.DT_CameraHeight" "Crouch")
                (:`then`
                  (set `self.newCameraHeight` (`.Height_2_0FCAD2D647485573C84BE993991DC84C` (break `/Game/_BattleRoyal/Blueprints/Data/Table/ST_CameraHeight` _returnvalue_3))))))))
        (elif (`/Game/_BattleRoyal/Blueprints/Character/BP_Character.isProne` _ownercharacter)
          (bind _returnvalue_4 (`|GetDataTableRow` "/Game/_BattleRoyal/Blueprints/Data/Table/DT_CameraHeight.DT_CameraHeight" "Prone")
            (:`then`
              (set `self.newCameraHeight` (`.Height_2_0FCAD2D647485573C84BE993991DC84C` (break `/Game/_BattleRoyal/Blueprints/Data/Table/ST_CameraHeight` _returnvalue_4)))))
          (else
            (bind _returnvalue_5 (`|GetDataTableRow` "/Game/_BattleRoyal/Blueprints/Data/Table/DT_CameraHeight.DT_CameraHeight" "Stand")
              (:`then`
                (set `self.newCameraHeight` (`.Height_2_0FCAD2D647485573C84BE993991DC84C` (break `/Game/_BattleRoyal/Blueprints/Data/Table/ST_CameraHeight` _returnvalue_5)))))))))
    (:`then_1`
      ;[1 1 1] Update Camera Height Location
      (if (!= _currentcameraheight (`self.newCameraHeight`))
        (set `self.originalCameraHeight` _currentcameraheight)
        (bind (_direction _percantage) (`Timeline|TL_UpateCameraHeight` :!via `PlayFromStart`)
          (:`Update`
            (bind _returnvalue_6 (`KismetMathLibrary.Lerp` (`self.originalCameraHeight`) (`self.newCameraHeight`) _percantage))
            (`SceneComponent.K2_SetRelativeLocation` _cameraboom (`KismetMathLibrary.MakeVector` _relativelocation_x _relativelocation_y _returnvalue_6) false false)
            (set `self.currentCameraHeight` _returnvalue_6)))))))

(event `self.ReceiveBeginPlay`
  (`WidgetBlueprintLibrary.SetInputMode_GameOnly` self)
  ;[1 1 1] Character Reference
  (bind _asbp_character (cast `/Game/_BattleRoyal/Blueprints/Character/BP_Character` (`GameplayStatics.GetPlayerCharacter` 0)))
  (set `self.OwnerCharacter` _asbp_character))

(event `InputAxis|Turn`
  (params (AxisValue :type "Float (single-precision)"))
  ;[1 1 1] Mouse Turn Left/Right
  (`/Game/_BattleRoyal/Blueprints/Character/BP_Character.MouseTurn` (`self.OwnerCharacter`) AxisValue))

(event `InputAxis|LookUp`
  (params (AxisValue :type "Float (single-precision)"))
  ;[1 1 1] Mouse Lookup/Down
  (bind _islimitcruss (`self.LimitPitchAngle` AxisValue))
  (if _islimitcruss
    (`/Game/_BattleRoyal/Blueprints/Character/BP_Character.MouseLookUp` (`self.OwnerCharacter`) AxisValue)))

(event `InputAxis|MoveForward`
  (params (AxisValue :type "Float (single-precision)"))
  ;[1 1 1] Move Left-Right / Backward-Forward
  (`|ExecutionSequence`
    (:`then_1`
      (if (`self.isEnableMove`)
        (bind _rotator (`self.Get Controller Rotation According to Alt Pressed`))
        (`self.MoveForwardBackward` true AxisValue _rotator)))))

(event `InputAxis|MoveRight`
  (params (AxisValue :type "Float (single-precision)"))
  ;[1 1 1] Move Left-Right / Backward-Forward
  (`|ExecutionSequence`
    (:`then_0`
      ;;[1 1 1] Update Camera Height
      (if (!= (`self.moveRightAxis`) AxisValue)
        (set `self.moveRightAxis` AxisValue)
        (`self.UpdateCameraHeight`)))
    (:`then_1`
      (if (`self.isEnableMove`)
        (`self.MoveForwardBackward` false AxisValue (stale `InputAxis|MoveForward` _rotator))))))

(event `self.ReceiveTick`
  (params (DeltaSeconds :type "Float (single-precision)"))
  (bind (_returnvalue_roll _returnvalue_pitch _returnvalue_yaw) (`KismetMathLibrary.BreakRotator` (`self.GetControlRotation`)))
  (`|ExecutionSequence`
    (:`then_0`
      ;[1 1 1] Rotation Character According to Move Turn
      (if (not (`self.isAltPressed`))
        (`self.K2_SetActorRotation` (`self.OwnerCharacter`) (`KismetMathLibrary.MakeRotator` 0.0 0.0 _returnvalue_yaw) false)))))

(event `InputAction|Alt`
  (params (Key :type "Key Structure"))
  (bind _returnvalue (`SpringArmComponent.GetTargetRotation` (`/Game/_BattleRoyal/Blueprints/Character/BP_Character.CameraBoom` (`self.OwnerCharacter`))))
  (:`Pressed`
    ;[1 1 1] Alt Key Pressed?
    (set `self.isAltPressed` true)
    ;[1 1 1] Alt Press Timeline Reply Function
    (set `self.altPressedRotation` _returnvalue))
  (:`Released`
    (set `self.Alt Released Rotation` _returnvalue)
    ;;[1 1 1] Camera Rotataion
    (bind (_direction _percentage) (`Timeline|TL_CameraRestore` :!via `PlayFromStart`)
      (:`Update`
        (`self.SetControlRotation` (`KismetMathLibrary.RLerp` (`self.Alt Released Rotation`) (`self.altPressedRotation`) _percentage true)))
      (:`Finished`
        (set `self.isAltPressed` false)))))

(event `InputAction|Crouch`
  (params (Key :type "Key Structure"))
  (bind _ownercharacter (`self.OwnerCharacter`))
  (:`Pressed`
    ;[1 1 1] Crouch/UnChrouch
    (`|ExecutionSequence`
      (:`then_0`
        (if (`/Game/_BattleRoyal/Blueprints/Character/BP_Character.isProne` _ownercharacter)
          (set `/Game/_BattleRoyal/Blueprints/Character/BP_Character.isProne` false _ownercharacter)
          (set `/Game/_BattleRoyal/Blueprints/Character/BP_Character.isCrouch` true _ownercharacter)
          (`self.HoldPosition` (`/Game/_BattleRoyal/Blueprints/Character/BP_Character.isHoldWeapon` _ownercharacter) "prone" "crouch")
          (elif (`/Game/_BattleRoyal/Blueprints/Character/BP_Character.isCrouch` _ownercharacter)
            (set `/Game/_BattleRoyal/Blueprints/Character/BP_Character.isCrouch` false _ownercharacter)
            (else
              (set `/Game/_BattleRoyal/Blueprints/Character/BP_Character.isCrouch` true _ownercharacter)))))
      (:`then_1`
        (`self.LimitPitchAngle` 0.0)
        (`self.UpdateCameraHeight`)))))

(event `InputAction|Prone`
  (params (Key :type "Key Structure"))
  (bind _ownercharacter (`self.OwnerCharacter`))
  (bind _isholdweapon (`/Game/_BattleRoyal/Blueprints/Character/BP_Character.isHoldWeapon` _ownercharacter))
  (:`Pressed`
    ;[1 1 1] Prone/UnProne
    (`|ExecutionSequence`
      (:`then_0`
        (if (`/Game/_BattleRoyal/Blueprints/Character/BP_Character.isProne` _ownercharacter)
          (set `/Game/_BattleRoyal/Blueprints/Character/BP_Character.isProne` false _ownercharacter)
          (`self.HoldPosition` _isholdweapon "prone" "stand")
          (elif (`/Game/_BattleRoyal/Blueprints/Character/BP_Character.isCrouch` _ownercharacter)
            (set `/Game/_BattleRoyal/Blueprints/Character/BP_Character.isCrouch` false _ownercharacter)
            (set `/Game/_BattleRoyal/Blueprints/Character/BP_Character.isProne` true _ownercharacter)
            (`self.HoldPosition` _isholdweapon "crouch" "prone")
            (else
              (set `/Game/_BattleRoyal/Blueprints/Character/BP_Character.isProne` true _ownercharacter)
              (`self.HoldPosition` _isholdweapon "stand" "prone")))))
      (:`then_1`
        (`self.LimitPitchAngle` 0.0)
        (`self.UpdateCameraHeight`)))))

(event `InputAction|Jump`
  (params (Key :type "Key Structure"))
  (bind _ownercharacter (`self.OwnerCharacter`))
  ;[1 1 1] Jump (When Prone/Crouch Then Chnage Normal Stand)
  (:`Pressed`
    (`|ExecutionSequence`
      (:`then_0`
        (if (or (`/Game/_BattleRoyal/Blueprints/Character/BP_Character.isProne` _ownercharacter) (`/Game/_BattleRoyal/Blueprints/Character/BP_Character.isCrouch` _ownercharacter))
          (set `/Game/_BattleRoyal/Blueprints/Character/BP_Character.isCrouch` false _ownercharacter)
          (set `/Game/_BattleRoyal/Blueprints/Character/BP_Character.isProne` false _ownercharacter)
          (else
            (`Character.Jump` _ownercharacter))))
      (:`then_1`
        (`self.UpdateCameraHeight`))))
  (:`Released`
    (`Character.StopJumping` _ownercharacter)))

(fn `Get Controller Rotation According to Alt Pressed`
  (returns (Rotator :type "Rotator Structure"))
  (if (`self.isAltPressed`)
    (return (`self.altPressedRotation`))
    (else
      (return (`self.GetControlRotation`)))))

(fn `LimitPitchAngle`
  (params (axis :type "Float (double-precision)"))
  (returns (isLimitCruss :type Boolean))
  (locals (b_value :type "Float (double-precision)") (t_value :type "Float (double-precision)"))
  (bind (_returnvalue_roll _returnvalue_pitch _returnvalue_yaw) (`KismetMathLibrary.BreakRotator` (`self.GetControlRotation`)))
  (bind (_returnvalue_roll_2 _returnvalue_pitch_2) (`KismetMathLibrary.BreakRotator` (`self.GetControlRotation`)))
  (bind (_returnvalue_roll_3 _returnvalue_pitch_3) (`KismetMathLibrary.BreakRotator` (`self.GetControlRotation`)))
  (bind _ownercharacter (`self.OwnerCharacter`))
  (bind _returnvalue (+ _returnvalue_pitch_2 (* (`local.axis`) (`self.input Pitch Scale`))))
  (`|ExecutionSequence`
    (:`then_0`
      ;[1 1 1] Calculate Axis Limit Value
      (if (`/Game/_BattleRoyal/Blueprints/Character/BP_Character.isProne` _ownercharacter)
        (set `local.b_value` 350.0)
        (set `local.t_value` 15.0)
        (elif (`/Game/_BattleRoyal/Blueprints/Character/BP_Character.isCrouch` _ownercharacter)
          (set `local.b_value` 290.0)
          (set `local.t_value` 50.0)
          (else
            (set `local.b_value` 290.0)
            (set `local.t_value` 75.0)))))
    (:`then_1`
      ;[1 1 1] If the limit is currently exceeded, set to the bounday value
      (if (or (> _returnvalue_pitch_3 (`local.b_value`)) (< _returnvalue_pitch_3 (`local.t_value`)))
        _
        (elif (< (`KismetMathLibrary.Abs` (- _returnvalue_pitch_3 (`local.t_value`))) (`KismetMathLibrary.Abs` (- _returnvalue_pitch_3 (`local.b_value`))))
          (`self.SetControlRotation` (`KismetMathLibrary.MakeRotator` _returnvalue_roll (`local.t_value`) _returnvalue_yaw))
          (else
            (`self.SetControlRotation` (`KismetMathLibrary.MakeRotator` _returnvalue_roll (`local.b_value`) _returnvalue_yaw))))))
    (:`then_2`
      ;[1 1 1] Determine if the limit is Cruss
      (return (or (> _returnvalue (`local.b_value`)) (< _returnvalue (`local.t_value`)))))))

(fn `MoveForwardBackward`
  (params (`is Forward` :type Boolean) (`axis Value` :type "Float (double-precision)") (controllerRotation :type "Rotator Structure"))
  (locals (NewLocalVar :type "Rotator Structure" :default (struct)))
  (bind _walkspeed (`self.walkSpeed`))
  (bind _ownercharacter (`self.OwnerCharacter`))
  (bind _returnvalue (`KismetMathLibrary.MakeRotator` 0.0 0.0 (.yaw controllerRotation)))
  (bind _charactermovement (`Character.CharacterMovement` (`self.OwnerCharacter`)))
  (bind _returnvalue_2 (+ (`KismetMathLibrary.VSize` (`MovementComponent.Velocity` _charactermovement)) 5.0))
  (if (<= _returnvalue_2 _walkspeed)
    (set `CharacterMovementComponent.MaxWalkSpeed` _returnvalue_2 _charactermovement)
    (else
      (set `CharacterMovementComponent.MaxWalkSpeed` _walkspeed _charactermovement)))
  (if `is Forward`
    (`Pawn.AddMovementInput` _ownercharacter (`KismetMathLibrary.GetForwardVector` _returnvalue) `axis Value` false)
    (else
      (`Pawn.AddMovementInput` _ownercharacter (`KismetMathLibrary.GetRightVector` _returnvalue) `axis Value` false))))

(fn `UserConstructionScript`)