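; Weapon item actor for the battle royale game, built from its DT_WeaponItems row by ID.
; The construction script sets the skeletal mesh and socket-attaches default magazine, muzzle, sight, foregrip and buttstock components.
; Update functions store each accessory and swap its mesh from DT_WeaponItemAccessories, reverting to default or empty when none is given.
; UpdateMagine is the exception: its check is inverted and its accessory mesh assignment is unwired.
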(fn `InitialDefaultWeaponAccessories`
  (params (`default Magine Static Mesh` :type "StaticMesh Object Reference") (`default Sight Mesh Static` :type "StaticMesh Object Reference") (`default Buttstock Static Mesh` :type "StaticMesh Object Reference") (Condition :type Boolean))
  (bind _skeletalmesh (`self.SkeletalMesh`))
  (bind _magine (`self.Magine`))
  (bind _sight (`self.Sight`))
  (bind _buttstock (`self.Buttstock`))
  (`|ExecutionSequence`
    (:`then_0`
      (`StaticMeshComponent.SetStaticMesh` _magine `default Magine Static Mesh`)
      (`SceneComponent.K2_AttachToComponent` _magine _skeletalmesh "Socket_Mag" "SnapToTarget" "KeepWorld" "KeepRelative" true))
    (:`then_1`
      (`SceneComponent.K2_AttachToComponent` (`self.Muzzle`) _skeletalmesh "Socket_Muzzle" "SnapToTarget" "KeepWorld" "KeepRelative" true))
    (:`then_2`
      (if (!= `default Sight Mesh Static` null)
        (`StaticMeshComponent.SetStaticMesh` _sight `default Sight Mesh Static`)
        (`SceneComponent.K2_AttachToComponent` _sight _skeletalmesh "Socket_Sight_Default" "SnapToTarget" "KeepWorld" "KeepRelative" true)))
    (:`then_3`
      (if Condition
        (`SceneComponent.K2_AttachToComponent` (`self.Foregrip`) _skeletalmesh "Socket_Foregrip" "SnapToTarget" "KeepWorld" "KeepRelative" true)))
    (:`then_4`
      (if (!= `default Buttstock Static Mesh` null)
        (`StaticMeshComponent.SetStaticMesh` _buttstock `default Buttstock Static Mesh`)
        (`SceneComponent.K2_AttachToComponent` _buttstock _skeletalmesh "Socket_Buttstock" "SnapToTarget" "KeepWorld" "KeepRelative" true)))))

(fn `UpdateButtstock`
  (params (buttstockAccesoriesActor :type "/Game/_BattleRoyal/Blueprints/Data/Equipments/BP_ItemWeaponAccessories Object Reference"))
  (bind (_datas_name _datas_icon _datas_bigicon _datas_thumbnail _datas_useammoid _datas_clipsize _datas_damge _datas_fringinterval _datas_replacecliptime _datas_replacebullettime _datas_isautomode _datas_staticmesh _datas_skeletalmesh _datas_defaultmagine _datas_defaultsight _datas_defaultbuttstock) (break `/Game/_BattleRoyal/Blueprints/Data/Table/ST_WeaponItems` (`self.datas`)))
  (bind _output_get (set `self.buttstockAccesoriesObject` buttstockAccesoriesActor))
  (if (== _output_get null)
    (`StaticMeshComponent.SetStaticMesh` (`self.Buttstock`) _datas_defaultbuttstock)
    (else
      (bind _returnvalue (`|GetDataTableRow` "/Game/_BattleRoyal/Blueprints/Data/Table/DT_WeaponItemAccessories.DT_WeaponItemAccessories" (`/Game/_BattleRoyal/Blueprints/Pickup/BP_ItemBase.ID` buttstockAccesoriesActor))
        (:`then`
          (`StaticMeshComponent.SetStaticMesh` (`self.Buttstock`) (`.StaticMesh_17_CCB843DB49D4518CE3A93EA5D35C0324` (break `/Game/_BattleRoyal/Blueprints/Data/Table/ST_WeaponItemAccessories` _returnvalue))))))))

(fn `UpdateForegrip`
  (params (foregripAccesoriesActor :type "/Game/_BattleRoyal/Blueprints/Data/Equipments/BP_ItemWeaponAccessories Object Reference"))
  (bind _output_get (set `self.foregripAccesoriesObject` foregripAccesoriesActor))
  (if (== _output_get null)
    (`StaticMeshComponent.SetStaticMesh` (`self.Foregrip`) null)
    (else
      (bind _returnvalue (`|GetDataTableRow` "/Game/_BattleRoyal/Blueprints/Data/Table/DT_WeaponItemAccessories.DT_WeaponItemAccessories" (`/Game/_BattleRoyal/Blueprints/Pickup/BP_ItemBase.ID` foregripAccesoriesActor))
        (:`then`
          (`StaticMeshComponent.SetStaticMesh` (`self.Foregrip`) (`.StaticMesh_17_CCB843DB49D4518CE3A93EA5D35C0324` (break `/Game/_BattleRoyal/Blueprints/Data/Table/ST_WeaponItemAccessories` _returnvalue))))))))

(fn `UpdateMagine`
  (params (magineAccesoriesActor :type "/Game/_BattleRoyal/Blueprints/Data/Equipments/BP_ItemWeaponAccessories Object Reference"))
  (bind (_datas_name _datas_icon _datas_bigicon _datas_thumbnail _datas_useammoid _datas_clipsize _datas_damge _datas_fringinterval _datas_replacecliptime _datas_replacebullettime _datas_isautomode _datas_staticmesh _datas_skeletalmesh _datas_defaultmagine) (break `/Game/_BattleRoyal/Blueprints/Data/Table/ST_WeaponItems` (`self.datas`)))
  (bind _output_get (set `self.accesesoriesMagineObj` magineAccesoriesActor))
  (if (!= _output_get null)
    (`StaticMeshComponent.SetStaticMesh` (`self.Magine`) _datas_defaultmagine)
    (else
      (bind _returnvalue (`|GetDataTableRow` "/Game/_BattleRoyal/Blueprints/Data/Table/DT_WeaponItemAccessories.DT_WeaponItemAccessories" (`self.ID`))))))

(fn `UpdateMuzzle`
  (params (muzzleAccesoriesActor :type "/Game/_BattleRoyal/Blueprints/Data/Equipments/BP_ItemWeaponAccessories Object Reference"))
  (bind _output_get (set `self.muzzleAccesoriesObject` muzzleAccesoriesActor))
  (if (== _output_get null)
    (`StaticMeshComponent.SetStaticMesh` (`self.Muzzle`) null)
    (else
      (bind _returnvalue (`|GetDataTableRow` "/Game/_BattleRoyal/Blueprints/Data/Table/DT_WeaponItemAccessories.DT_WeaponItemAccessories" (`/Game/_BattleRoyal/Blueprints/Pickup/BP_ItemBase.ID` _output_get))
        (:`then`
          (`StaticMeshComponent.SetStaticMesh` (`self.Muzzle`) (`.StaticMesh_17_CCB843DB49D4518CE3A93EA5D35C0324` (break `/Game/_BattleRoyal/Blueprints/Data/Table/ST_WeaponItemAccessories` _returnvalue))))))))

(fn `UpdateSight`
  (params (sightAccesoriesActor :type "/Game/_BattleRoyal/Blueprints/Data/Equipments/BP_ItemWeaponAccessories Object Reference"))
  (bind (_datas_name _datas_icon _datas_bigicon _datas_thumbnail _datas_useammoid _datas_clipsize _datas_damge _datas_fringinterval _datas_replacecliptime _datas_replacebullettime _datas_isautomode _datas_staticmesh _datas_skeletalmesh _datas_defaultmagine _datas_defaultsight) (break `/Game/_BattleRoyal/Blueprints/Data/Table/ST_WeaponItems` (`self.datas`)))
  (bind _output_get (set `self.sightAccesoriesObject` sightAccesoriesActor))
  (if (== _output_get null)
    (`StaticMeshComponent.SetStaticMesh` (`self.Sight`) _datas_defaultsight)
    (`SceneComponent.K2_AttachToComponent` (`self.Sight`) (`self.SkeletalMesh`) "Socket_Sight_Default" "KeepRelative" "KeepRelative" "KeepRelative" true)
    (else
      (bind _returnvalue (`|GetDataTableRow` "/Game/_BattleRoyal/Blueprints/Data/Table/DT_WeaponItemAccessories.DT_WeaponItemAccessories" (`/Game/_BattleRoyal/Blueprints/Pickup/BP_ItemBase.ID` sightAccesoriesActor))
        (:`then`
          (`StaticMeshComponent.SetStaticMesh` (`self.Sight`) (`.StaticMesh_17_CCB843DB49D4518CE3A93EA5D35C0324` (break `/Game/_BattleRoyal/Blueprints/Data/Table/ST_WeaponItemAccessories` _returnvalue)))
          (`SceneComponent.K2_AttachToComponent` (`self.Sight`) (`self.SkeletalMesh`) (`.SocketName_49_FA6CD1E846757F02D4C0BEA3B12EDA62` (break `/Game/_BattleRoyal/Blueprints/Data/Table/ST_WeaponItemAccessories` _returnvalue)) "KeepRelative" "KeepRelative" "KeepRelative" true))))))

(fn `UserConstructionScript`
  (bind _returnvalue (`|GetDataTableRow` "/Game/_BattleRoyal/Blueprints/Data/Table/DT_WeaponItems.DT_WeaponItems" (`self.ID`))
    (:`then`
      (bind _output_get (set `self.datas` _returnvalue))
      (bind (_name _icon _bigicon _thumbnail _useammoid _clipsize _damge _fringinterval _replacecliptime _replacebullettime _isautomode _staticmesh _skeletalmesh _defaultmagine _defaultsight _defaultbuttstock _firesound _firesoundsuppressor _issight _ismuzzle _isclip _isbuttstock _isgrip) (break `/Game/_BattleRoyal/Blueprints/Data/Table/ST_WeaponItems` _output_get))
      (`self.Initilaze` "NewEnumerator0" _name)
      ;[1 1 1] Set the weapon skeletal mesh
      (`SkeletalMeshComponent.SetSkeletalMeshAsset` (`self.SkeletalMesh`) _skeletalmesh)
      ;[1 1 1] Set Default Weapon Accessorires.
      (`self.InitialDefaultWeaponAccessories` _defaultmagine _defaultsight _defaultbuttstock _isgrip))))