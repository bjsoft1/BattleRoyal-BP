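; Battle royale player character with modular clothing and display of carried weapons and equipment.
; Clothing meshes follow the body's pose and come from DT_FashionItems, with mask textures on a dynamic skin material and underwear fallbacks for empty top or bottom slots.
; Display functions read PlayerState and attach items to GameInstance-named sockets, choosing back sockets by backpack and hiding hair under helmets.
; Number keys trigger hard-coded test weapon spawning and outfit swaps.
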(event `self.ReceiveBeginPlay`
  ;[1 1 1] Reference Variable Initialize
  (bind _asbp_player_state (cast `/Game/_BattleRoyal/Blueprints/Game/BP_PlayerState` (`GameplayStatics.GetPlayerState` 0)))
  (set `self.playerStateReference` _asbp_player_state)
  (bind _asbp_game_instance (cast `/Game/_BattleRoyal/Blueprints/Game/BP_GameInstance` (`GameplayStatics.GetGameInstance`)))
  (set `self.gameInstanceRefernce` _asbp_game_instance))

(event `Key|One`
  (params (Key :type "Key Structure"))
  (:`Pressed`
    (set `self.isHoldWeapon` true)
    (bind _returnvalue (`|SpawnActorFromClass` "/Game/_BattleRoyal/Blueprints/Pickup/Equipments/BP_ItemWeapon.BP_ItemWeapon_C" (`KismetMathLibrary.MakeTransform` (0.0 0.0 0.0)) "Undefined" "OverrideRootScale" null 0 false "111" "1" 1 null))
    (`/Game/_BattleRoyal/Blueprints/Game/BP_PlayerState.SetHoldWeapon` (`self.playerStateReference`) _returnvalue)))

(event `Key|Two`
  (params (Key :type "Key Structure"))
  (:`Pressed`
    (`self.ChangeSkeletalMesh` "NewEnumerator0" "2")))

(event `Key|Three`
  (params (Key :type "Key Structure"))
  (:`Pressed`
    (`self.ChangeSkeletalMesh` "NewEnumerator0" "3")))

(event `Key|Four`
  (params (Key :type "Key Structure"))
  (:`Pressed`
    (`self.ChangeSkeletalMesh` "NewEnumerator1" "0")))

(event `Key|Five`
  (params (Key :type "Key Structure"))
  (:`Pressed`
    (`self.ChangeSkeletalMesh` "NewEnumerator1" "5")))

(event `Key|Six`
  (params (Key :type "Key Structure"))
  (:`Pressed`
    (`self.ChangeSkeletalMesh` "NewEnumerator1" "6")))

(event `Key|Seven`
  (params (Key :type "Key Structure"))
  (:`Pressed`
    (`self.ChangeSkeletalMesh` "NewEnumerator2" "0")))

(event `Key|Eight`
  (params (Key :type "Key Structure"))
  (:`Pressed`
    (`self.ChangeSkeletalMesh` "NewEnumerator2" "7")))

(event `Key|Zero`
  (params (Key :type "Key Structure"))
  (:`Pressed`
    (`self.ChangeSkeletalMesh` "NewEnumerator3" "8")))

(event `Key|Nine`
  (params (Key :type "Key Structure"))
  (:`Pressed`
    (`self.ChangeSkeletalMesh` "NewEnumerator3" "0")))

(fn `AttachActor`
  (params (item :type "/Game/_BattleRoyal/Blueprints/Pickup/BP_ItemBase Object Reference") (socketName :type Name))
  (`self.K2_SetActorTransform` item (`SceneComponent.GetSocketTransform` (`self.Mesh`) socketName "RTS_World") false false)
  (`self.K2_AttachToComponent` item (`self.Mesh`) socketName "SnapToTarget" "KeepWorld" "KeepRelative" true))

(fn `ChangeSkeletalMesh`
  (params (fashionType :type "/Game/_BattleRoyal/Blueprints/Data/Enum/E_FashionTypes Enum" :default "NewEnumerator0") (name :type Name))
  (locals (skm :type "SkeletalMesh Object Reference") (maskTexture :type "Texture Object Reference"))
  (bind _masktexture (`local.maskTexture`))
  (bind _skinmaterialreference (`self.skinMaterialReference`))
  (bind _skinmaterialreference_2 (`self.skinMaterialReference`))
  (bind _mesh (`self.Mesh`))
  (bind _skm (`local.skm`))
  (`|ExecutionSequence`
    (:`then_0`
      (bind (_skeletalmesh _masktexture_2) (`self.GetFashionRowByName` name))
      (set `local.skm` _skeletalmesh)
      (set `local.maskTexture` _masktexture_2)
      ;[1 1 1] Change Fashion Skeletal Mesh
      (switch `/Game/_BattleRoyal/Blueprints/Data/Enum/E_FashionTypes` fashionType
        (:`NewEnumerator0`
          (`SkeletalMeshComponent.SetSkeletalMeshAsset` (`self.SKM_ClothTop`) _skm)
          ;[1 1 1] Update Material According to Dress
          (`MaterialInstanceDynamic.SetTextureParameterValue` _skinmaterialreference_2 "Mask Top" _masktexture)
          ;[1 1 1] Remove After Changing Clothing Unnesarray Choths
          (if (!= _skm null)
            (`SkeletalMeshComponent.SetSkeletalMeshAsset` (`self.SKM_Whole`) null)))
        (:`NewEnumerator1`
          (`SkeletalMeshComponent.SetSkeletalMeshAsset` (`self.SKM_ClothButtom`) _skm)
          (`MaterialInstanceDynamic.SetTextureParameterValue` _skinmaterialreference_2 "Mask Bottom" _masktexture)
          (if (!= _skm null)
            (`SkeletalMeshComponent.SetSkeletalMeshAsset` (`self.SKM_Whole`) null)))
        (:`NewEnumerator2`
          (`SkeletalMeshComponent.SetSkeletalMeshAsset` (`self.SKM_Whole`) _skm)
          (`MaterialInstanceDynamic.SetTextureParameterValue` _skinmaterialreference_2 "Mask Top" _masktexture)
          (if (!= _skm null)
            (`SkeletalMeshComponent.SetSkeletalMeshAsset` (`self.SKM_ClothTop`) null)
            (`SkeletalMeshComponent.SetSkeletalMeshAsset` (`self.SKM_ClothButtom`) null)))
        (:`NewEnumerator3`
          (`SkeletalMeshComponent.SetSkeletalMeshAsset` (`self.SKM_Shoes`) _skm)
          (`/Engine/EditorBlueprintResources/StandardMacros.IsValid` _skm
            (:`Is Valid`
              (`MaterialInstanceDynamic.SetTextureParameterValue` _skinmaterialreference_2 "Mask Foot" _masktexture)
              ;[1 1 1] Change Character Mesh Height Location When ware Shoes
              (`SceneComponent.K2_SetRelativeLocation` _mesh (0.0 0.0 -96.9) false false))
            (:`Is Not Valid`
              (`MaterialInstanceDynamic.SetTextureParameterValue` _skinmaterialreference_2 "Mask Foot" "/Game/Assets/Humans/Female/Textures/System/TX_Empty_white.TX_Empty_white")
              (`SceneComponent.K2_SetRelativeLocation` _mesh (0.0 0.0 -97.6) false false))))))
    (:`then_1`
      ;[1 1 1] Remove Materail Mask According to new Cloths
      (`/Engine/EditorBlueprintResources/StandardMacros.IsValid` (`SkeletalMeshComponent.SkeletalMeshAsset` (`self.SKM_Whole`))
        (:`Is Valid`
          (`MaterialInstanceDynamic.SetTextureParameterValue` _skinmaterialreference "Mask Bottom" "/Game/Assets/Humans/Female/Textures/System/TX_Empty_white.TX_Empty_white"))
        (:`Is Not Valid`
          (`|ExecutionSequence`
            (:`then_0`
              (`/Engine/EditorBlueprintResources/StandardMacros.IsValid` (`SkeletalMeshComponent.SkeletalMeshAsset` (`self.SKM_ClothTop`))
                (:`Is Not Valid`
                  (bind (_skeletalmesh_2 _masktexture_3) (`self.GetFashionRowByName` "1"))
                  ;;[1 1 1] Set Default Underware Mesh
                  (`SkeletalMeshComponent.SetSkeletalMeshAsset` (`self.SKM_ClothTop`) _skeletalmesh_2)
                  (`MaterialInstanceDynamic.SetTextureParameterValue` _skinmaterialreference "Mask Top" _masktexture_3))))
            (:`then_1`
              (`/Engine/EditorBlueprintResources/StandardMacros.IsValid` (`SkeletalMeshComponent.SkeletalMeshAsset` (`self.SKM_ClothButtom`))
                (:`Is Not Valid`
                  (bind (_skeletalmesh_3 _masktexture_4) (`self.GetFashionRowByName` "4"))
                  (`SkeletalMeshComponent.SetSkeletalMeshAsset` (`self.SKM_ClothButtom`) _skeletalmesh_3)
                  (`MaterialInstanceDynamic.SetTextureParameterValue` _skinmaterialreference "Mask Bottom" _masktexture_4))))))))))

(fn `ClearFashion`
  (`self.ChangeSkeletalMesh` "NewEnumerator0" "0")
  (`self.ChangeSkeletalMesh` "NewEnumerator1" "0")
  (`self.ChangeSkeletalMesh` "NewEnumerator2" "0")
  (`self.ChangeSkeletalMesh` "NewEnumerator3" "0"))

(fn `GetFashionRowByName`
  (params (Id :type Name))
  (returns (skeletalMesh :type "SkeletalMesh Object Reference") (maskTexture :type "Texture Object Reference"))
  (bind _returnvalue (`|GetDataTableRow` "/Game/_BattleRoyal/Blueprints/Data/Table/DT_FashionItems.DT_FashionItems" Id)
    (:`then`
      (bind (_type _name _icon _skeletalmesh _staticmesh _masktexture) (break `/Game/_BattleRoyal/Blueprints/Data/Table/ST_FashionTypes` _returnvalue))
      (return _skeletalmesh _masktexture))
    (:`RowNotFound`
      (return null null))))

(fn `InitialSkeletalMesh`
  (`|ExecutionSequence`
    (:`then_0`
      ;[1 1 1] Create skin Material
      (bind _returnvalue (`KismetMaterialLibrary.CreateDynamicMaterialInstance` "/Game/Assets/Humans/Female/Materials/Skin/M_MT_Skin.M_MT_Skin"))
      (bind _output_get (set `self.skinMaterialReference` _returnvalue))
      (`PrimitiveComponent.SetMaterialByName` (`self.Mesh`) "skin" _output_get))
    (:`then_1`
      ;[1 1 1] Set master pose
      (`SkinnedMeshComponent.SetLeaderPoseComponent` (`self.SKM_Shoes`) (`self.Mesh`) false false)
      (`SkinnedMeshComponent.SetLeaderPoseComponent` (`self.SKM_Whole`) (`self.Mesh`) false false)
      (`SkinnedMeshComponent.SetLeaderPoseComponent` (`self.SKM_ClothButtom`) (`self.Mesh`) false false)
      (`SkinnedMeshComponent.SetLeaderPoseComponent` (`self.SKM_ClothTop`) (`self.Mesh`) false false)
      (`SkinnedMeshComponent.SetLeaderPoseComponent` (`self.SKM_UnderwareButtom`) (`self.Mesh`) false false)
      (`SkinnedMeshComponent.SetLeaderPoseComponent` (`self.SKM_UnderwareTop`) (`self.Mesh`) false false)
      ;[1 1 1] Attach Hair
      (`SceneComponent.K2_AttachToComponent` (`self.SKM_Hair`) (`self.Mesh`) "HairSocket" "KeepRelative" "KeepRelative" "KeepRelative" false)
      ;[1 1 1] Set Default Cloth (Underware)
      (`self.ChangeSkeletalMesh` "NewEnumerator0" "0"))))

(fn `MouseLookUp`
  (params (`axis Value` :type "Float (double-precision)"))
  (`self.AddControllerPitchInput` `axis Value`))

(fn `MouseTurn`
  (params (`axis Value` :type "Float (double-precision)"))
  (`self.AddControllerYawInput` `axis Value`))

(fn `Update Fashion Display`
  (`self.ClearFashion`)
  (for _array_element (`/Game/_BattleRoyal/Blueprints/Game/BP_PlayerState.GetFashioons` (`self.playerStateReference`))
    (bind _asbp_pickup_fashion (cast `/Game/_BattleRoyal/Blueprints/Pickup/BP_PickupFashion` _array_element))
    (`self.ChangeSkeletalMesh` (`/Game/_BattleRoyal/Blueprints/Pickup/BP_PickupFashion.fashionType` _asbp_pickup_fashion) (`/Game/_BattleRoyal/Blueprints/Pickup/BP_ItemBase.ID` _asbp_pickup_fashion))))

(fn `UpdateEquipmentDisplay`
  (locals (item :type "/Game/_BattleRoyal/Blueprints/Pickup/BP_ItemBase Object Reference") (isHelmet :type Boolean))
  (`|ExecutionSequence`
    (:`then_0`
      (for _array_element (`/Game/_BattleRoyal/Blueprints/Game/BP_PlayerState.GetEquipments` (`self.playerStateReference`))
        (bind _output_get (set `local.item` _array_element))
        (switch `/Game/_BattleRoyal/Blueprints/Data/Enum/E_ItemType` (`/Game/_BattleRoyal/Blueprints/Pickup/BP_ItemBase.ItemType` _output_get)
          (:`NewEnumerator5`
            (`self.AttachActor` (`local.item`) (`/Game/_BattleRoyal/Blueprints/Game/BP_GameInstance.HelmetName` (`self.gameInstanceRefernce`)))
            (set `local.isHelmet` true))
          (:`NewEnumerator6`
            (`self.AttachActor` (`local.item`) (`/Game/_BattleRoyal/Blueprints/Game/BP_GameInstance.VestName` (`self.gameInstanceRefernce`))))
          (:`NewEnumerator7`
            (`self.AttachActor` (`local.item`) (`/Game/_BattleRoyal/Blueprints/Game/BP_GameInstance.BackpackName` (`self.gameInstanceRefernce`)))))))
    (:`then_1`
      (`SceneComponent.SetVisibility` (`self.SKM_Hair`) (not (`local.isHelmet`)) false))))

(fn `UpdateWeaponDisplay`
  (params (holdSocket :type Name))
  (locals (isBackpack :type Boolean))
  (bind _gameinstancerefernce (`self.gameInstanceRefernce`))
  (bind _gameinstancerefernce_2 (`self.gameInstanceRefernce`))
  (bind _playerstatereference (`self.playerStateReference`))
  (bind _weapon (`/Game/_BattleRoyal/Blueprints/Game/BP_PlayerState.GetWeapon1` _playerstatereference))
  (bind _weapon_2 (`/Game/_BattleRoyal/Blueprints/Game/BP_PlayerState.GetWeapon2` _playerstatereference))
  (bind _weapon_3 (`/Game/_BattleRoyal/Blueprints/Game/BP_PlayerState.GetHoldWeapon` (`self.playerStateReference`)))
  (`|ExecutionSequence`
    (:`then_0`
      ;[1 1 1] Update the handle weapon display
      (if (!= holdSocket "None")
        (`/Engine/EditorBlueprintResources/StandardMacros.IsValid` _weapon_3
          (:`Is Valid`
            (`self.AttachActor` _weapon_3 (`local.holdSocket`))))))
    (:`then_1`
      (`|ExecutionSequence`
        (:`then_0`
          (for _array_element (`/Game/_BattleRoyal/Blueprints/Game/BP_PlayerState.GetEquipments` _playerstatereference)
            (if (`|EnumEquality` (`/Game/_BattleRoyal/Blueprints/Pickup/BP_ItemBase.ItemType` _array_element) "NewEnumerator7")
              (set `local.isBackpack` true))))
        (:`then_1`
          ;[1 1 1] Update Back Weapon display location
          (`/Engine/EditorBlueprintResources/StandardMacros.IsValid` (`/Game/_BattleRoyal/Blueprints/Game/BP_PlayerState.GetWeapon1` _playerstatereference)
            (:`Is Valid`
              (if (`local.isBackpack`)
                (`self.AttachActor` _weapon (`/Game/_BattleRoyal/Blueprints/Game/BP_GameInstance.BackLeft_B_Name` _gameinstancerefernce_2))
                (else
                  (`self.AttachActor` _weapon (`/Game/_BattleRoyal/Blueprints/Game/BP_GameInstance.BackLeft_N_Name` _gameinstancerefernce_2)))))))
        (:`then_2`
          (`/Engine/EditorBlueprintResources/StandardMacros.IsValid` _weapon_2
            (:`Is Valid`
              (if (`local.isBackpack`)
                (`self.AttachActor` _weapon_2 (`/Game/_BattleRoyal/Blueprints/Game/BP_GameInstance.BackRight_B_Name` _gameinstancerefernce))
                (else
                  (`self.AttachActor` _weapon_2 (`/Game/_BattleRoyal/Blueprints/Game/BP_GameInstance.BackRight_N_Name` _gameinstancerefernce)))))))))))

(fn `UserConstructionScript`
  (`self.InitialSkeletalMesh`))